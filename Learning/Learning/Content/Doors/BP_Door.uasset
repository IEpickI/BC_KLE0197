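; BP_Door is a hinged door actor that toggles between closed and open when OpenDoor is called.
; A FlipFlop plays or reverses a timeline that lerps the door mesh yaw from shut to a quarter turn.
; A sphere overlap shows or hides the Interaction widget, which GetWidget exposes to callers.
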(event `Open Door`
  (`/Engine/EditorBlueprintResources/StandardMacros.FlipFlop`
    (:`A`
      (bind (_direction _output) (`Timeline|TimeLine` :!label _label)
        (:`Update`
          (`SceneComponent.K2_SetRelativeRotation` (`self.Door`) (`KismetMathLibrary.MakeRotator` 0.0 0.0 (`KismetMathLibrary.Lerp` 0.0 90.0 _output)) false false))))
    (:`B`
      (goto _label :!via `Reverse`))))

(event `self.Sphere.OnComponentBeginOverlap`
  (params (OverlappedComponent :type "PrimitiveComponent Object Reference") (OtherActor :type "Actor Object Reference") (OtherComp :type "PrimitiveComponent Object Reference") (OtherBodyIndex :type Integer) (bFromSweep :type Boolean) (SweepResult :type "HitResult Structure (by ref)"))
  (`SceneComponent.SetVisibility` (`self.Interaction`) true false))

(event `self.Sphere.OnComponentEndOverlap`
  (params (OverlappedComponent :type "PrimitiveComponent Object Reference") (OtherActor :type "Actor Object Reference") (OtherComp :type "PrimitiveComponent Object Reference") (OtherBodyIndex :type Integer))
  (`SceneComponent.SetVisibility` (`self.Interaction`) false false))

(fn `GetWidget`
  (returns (NewParam :type "WidgetComponent Object Reference"))
  (return (`self.Interaction`)))

(fn `UserConstructionScript`)