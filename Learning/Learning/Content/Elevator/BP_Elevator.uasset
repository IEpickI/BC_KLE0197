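; Elevator actor that lifts its platform and carries the player on to the level "NewLevel".
; A box overlap enables input and shows an interaction prompt, and F flip-flops a Timeline between play and reverse to lerp the platform's relative height.
; While the Timeline output exceeds halfway, each update casts the pawn to BP_ThirdPersonCharacter, spawns a new WB_Transition widget and opens the level after a short delay.
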(event `self.Box.OnComponentBeginOverlap`
  (params (OverlappedComponent :type "PrimitiveComponent Object Reference") (OtherActor :type "Actor Object Reference") (OtherComp :type "PrimitiveComponent Object Reference") (OtherBodyIndex :type Integer) (bFromSweep :type Boolean) (SweepResult :type "HitResult Structure (by ref)"))
  (`self.EnableInput` (`GameplayStatics.GetPlayerController` 0))
  (`SceneComponent.SetVisibility` (`self.Interaction`) true false))

(event `self.Box.OnComponentEndOverlap`
  (params (OverlappedComponent :type "PrimitiveComponent Object Reference") (OtherActor :type "Actor Object Reference") (OtherComp :type "PrimitiveComponent Object Reference") (OtherBodyIndex :type Integer))
  (`self.DisableInput` (`GameplayStatics.GetPlayerController` 0))
  (`SceneComponent.SetVisibility` (`self.Interaction`) false false))

(event `Key|F`
  (params (Key :type "Key Structure"))
  (:`Pressed`
    (`/Engine/EditorBlueprintResources/StandardMacros.FlipFlop`
      (:`A`
        (bind (_direction _output) (`Timeline|Timeline` :!label _label)
          (:`Update`
            (`SceneComponent.K2_SetRelativeLocation` (`self.Elevator`) (`KismetMathLibrary.MakeVector` 0.0 0.0 (`KismetMathLibrary.Lerp` 0.0 950.0 _output)) false false)
            (if (> _output 0.5)
              (cast `/Game/ThirdPerson/Blueprints/BP_ThirdPersonCharacter` (`GameplayStatics.GetPlayerPawn` 0))
              (bind _returnvalue (`|CreateWidget` "/Game/Elevator/WB_Transition.WB_Transition_C"))
              (`UserWidget.AddToViewport` _returnvalue 0)
              (`/Game/Elevator/WB_Transition.Transition_Event` _returnvalue)
              (`KismetSystemLibrary.Delay` 0.5)
              (`GameplayStatics.OpenLevel` "NewLevel")))))
      (:`B`
        (goto _label :!via `Reverse`)))))

(fn `UserConstructionScript`)